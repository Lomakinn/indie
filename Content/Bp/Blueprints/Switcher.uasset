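; Switcher is a one-way switch that the CH_Player character trips by overlapping its Box component.
; The overlap calls Activate on the player's root component and the Box, and the Box's OnComponentActivated event sets IsActivated, which nothing here clears during play.
; Tick swaps a construction-script-created, collision-free Paper2D sprite between on and off art to match that flag.
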(event `self.ReceiveTick`
  (params (DeltaSeconds :type "Float (single-precision)"))
  (bind _spritecomp (`self.SpriteComp`))
  (if (`self.IsActivated`)
    (`PaperSpriteComponent.SetSprite` _spritecomp (`self.OnSprite`))
    (else
      (`PaperSpriteComponent.SetSprite` _spritecomp (`self.OffSprite`)))))

(event `self.Box.OnComponentActivated`
  (params (Component :type "ActorComponent Object Reference") (bReset :type Boolean))
  (set `self.IsActivated` true))

(event `self.Box.OnComponentBeginOverlap`
  (params (OverlappedComponent :type "PrimitiveComponent Object Reference") (OtherActor :type "Actor Object Reference") (OtherComp :type "PrimitiveComponent Object Reference") (OtherBodyIndex :type Integer) (bFromSweep :type Boolean) (SweepResult :type "HitResult Structure (by ref)"))
  (bind _asch_player (cast `/Game/Bp/Blueprints/CH_Player` OtherActor))
  (`ActorComponent.Activate` (`Actor.RootComponent` _asch_player) false)
  (`ActorComponent.Activate` OverlappedComponent false))

(fn `UserConstructionScript`
  (bind _returnvalue (`AddComponent|NODE_AddPaperSpriteComponent-4`))
  (set `self.IsActivated` false)
  (bind _output_get (set `self.SpriteComp` _returnvalue))
  (`PrimitiveComponent.SetCollisionEnabled` _output_get "NoCollision"))