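; A climbable Paper2D ladder whose height comes from the Z distance between LadderBottom and LadderTop.
; The construction script stacks collision-free rung sprites at RungOffset spacing and stretches and shifts the Box trigger to that height.
; Box overlap toggles IsCanClimb on CH_Player and calls ClimbingEnd on exit.
; SwitchState adds another rung stack using LadderSprite02, without removing existing sprites.
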(event `self.Box.OnComponentBeginOverlap`
  (params (OverlappedComponent :type "PrimitiveComponent Object Reference") (OtherActor :type "Actor Object Reference") (OtherComp :type "PrimitiveComponent Object Reference") (OtherBodyIndex :type Integer) (bFromSweep :type Boolean) (SweepResult :type "HitResult Structure (by ref)"))
  (bind _asch_player (cast `/Game/Bp/Blueprints/CH_Player` OtherActor))
  (set `/Game/Bp/Blueprints/CH_Player.IsCanClimb` true _asch_player))

(event `self.Box.OnComponentEndOverlap`
  (params (OverlappedComponent :type "PrimitiveComponent Object Reference") (OtherActor :type "Actor Object Reference") (OtherComp :type "PrimitiveComponent Object Reference") (OtherBodyIndex :type Integer))
  (bind _asch_player (cast `/Game/Bp/Blueprints/CH_Player` OtherActor))
  (set `/Game/Bp/Blueprints/CH_Player.IsCanClimb` false _asch_player)
  (`/Game/Bp/Blueprints/CH_Player.ClimbingEnd` _asch_player))

(fn `SwitchState`
  (bind _rungoffset (`self.RungOffset`))
  (bind (_returnvalue_x _returnvalue_y _returnvalue_z) (`KismetMathLibrary.BreakVector` (- (`self.LadderTop`) (`self.LadderBottom`))))
  (for _index (range (+ (`KismetMathLibrary.FTrunc` (/ _returnvalue_z _rungoffset)) 1))
    (bind _returnvalue (`AddComponent|NODE_AddPaperSpriteComponent-2` :`RelativeTransform` (`KismetMathLibrary.MakeTransform` (`KismetMathLibrary.MakeVector` 0.0 0.0 (* _index _rungoffset)))))
    (`PaperSpriteComponent.SetSprite` _returnvalue (`self.LadderSprite02`))
    (`PrimitiveComponent.SetCollisionEnabled` _returnvalue "NoCollision")))

(fn `UserConstructionScript`
  (bind _box (`self.Box`))
  (bind _rungoffset (`self.RungOffset`))
  (bind (_returnvalue_x _returnvalue_y _returnvalue_z) (`KismetMathLibrary.BreakVector` (- (`self.LadderTop`) (`self.LadderBottom`))))
  (bind _returnvalue (/ _returnvalue_z 2.0))
  (for _index (range (+ (`KismetMathLibrary.FTrunc` (/ _returnvalue_z _rungoffset)) 1))
    (bind _returnvalue_2 (`AddComponent|NODE_AddPaperSpriteComponent-0` :`RelativeTransform` (`KismetMathLibrary.MakeTransform` (`KismetMathLibrary.MakeVector` 0.0 0.0 (* _index _rungoffset)))))
    (`PaperSpriteComponent.SetSprite` _returnvalue_2 (`self.LadderSprite`))
    (`PrimitiveComponent.SetCollisionEnabled` _returnvalue_2 "NoCollision"))
  (`SceneComponent.SetRelativeScale3D` _box (`KismetMathLibrary.MakeVector` 1.0 1.0 _returnvalue))
  (`SceneComponent.K2_AddRelativeLocation` _box (`KismetMathLibrary.MakeVector` 1.0 1.0 _returnvalue) false false))