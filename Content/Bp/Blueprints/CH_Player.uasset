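; CH_Player is a 2D flipbook player character with side movement, ladder-style climbing and an unfinished attack.
; MoveUp switches movement to Flying while climbing is allowed, pausing the flipbook without input; ClimbingEnd restores Walking.
; Tick selects flipbooks through a priority-based state function and rotates the sprite by velocity; every state except Running uses ClimbingGirl.
; Fire sets IsAttacking, never cleared here, then calls an empty FireProjectile after a delay.
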(event `self.ReceiveBeginPlay`
  (`ActorComponent.SetIsReplicated` (`self.Sprite`) true))

(event `UpdateAnimation`
  ;[1 1 1] Handle Animation
  (bind _output_get (set `self.IsMoving` (> (`KismetMathLibrary.VSize` (`self.GetVelocity`)) 0.0)))
  (bind _outputfb (`self.AnimationStateMachine` _output_get (`self.IsFalling`) (`self.IsAttacking`) (`self.IsClimbing`)))
  (`PaperFlipbookComponent.SetFlipbook` (`self.Sprite`) _outputfb))

(event `InputAxis|MoveRight`
  (params (AxisValue :type "Float (single-precision)"))
  ;[1 1 1] Handle movement
  (if (`self.CanMoveRight`)
    (`self.AddMovementInput` (1.0 0.0 0.0) AxisValue)))

(event `self.ReceiveTick`
  (params (DeltaSeconds :type "Float (single-precision)"))
  (bind _sprite (`self.Sprite`))
  (bind _sprite_2 (`self.Sprite`))
  ;[1 1 1] Tick - Updates animation
  (`self.UpdateAnimation`)
  (`|ExecutionSequence`
    (:`then_0`
      (`/Engine/EditorBlueprintResources/StandardMacros.CompareFloat` (.x (`MovementComponent.Velocity` (`self.CharacterMovement`)))
        (:`>`
          (`SceneComponent.K2_SetRelativeRotation` :`self` _sprite_2))
        (:`<`
          (`SceneComponent.K2_SetRelativeRotation` _sprite_2 (struct :`Yaw` 180.0) false false))))
    (:`then_1`
      (`/Engine/EditorBlueprintResources/StandardMacros.CompareFloat` (.z (`MovementComponent.Velocity` (`self.CharacterMovement`)))
        (:`>`
          (`SceneComponent.K2_SetRelativeRotation` :`self` _sprite))
        (:`<`
          (`SceneComponent.K2_SetRelativeRotation` _sprite (struct :`Roll` 180.0) false false))))))

(event `InputAxis|MoveUp`
  (params (AxisValue :type "Float (single-precision)"))
  (bind _sprite (`self.Sprite`))
  ;[1 1 1] Handle Climbing
  (if (`self.IsCanClimb`)
    (if (`KismetMathLibrary.InRange_FloatFloat` AxisValue -0.1 0.1)
      (`PaperFlipbookComponent.SetPlayRate` _sprite 0.0)
      (else
        (set `self.IsClimbing` true)
        (set `self.CanMoveRight` true)
        (`PaperFlipbookComponent.SetPlayRate` _sprite 1.0)
        (`CharacterMovementComponent.SetMovementMode` (`self.CharacterMovement`) "MOVE_Flying" 0)
        (`self.AddMovementInput` (0.0 0.0 0.5) AxisValue)))))

(event `ClimbingEnd`
  ;[1 1 1] Handle Climbing
  (if (`self.IsClimbing`)
    (`CharacterMovementComponent.SetMovementMode` (`self.CharacterMovement`) "MOVE_Walking" 0)
    (set `self.IsClimbing` false)
    (set `self.CanMoveRight` true)
    (`PaperFlipbookComponent.SetPlayRate` (`self.Sprite`) 1.0)))

(event `InputAction|FIre`
  (params (Key :type "Key Structure"))
  (:`Pressed`
    (if (not (`self.IsAttacking`))
      (`self.AttackAnimation`))))

(event `AttackAnimation`
  (`|ExecutionSequence`
    (:`then_0`
      (set `self.IsAttacking` true)
      (`KismetSystemLibrary.Delay` 0.3)
      (`self.FireProjectile`))))

(event `FireProjectile`)

(fn `AnimationStateMachine`
  (params (IsMoving :type Boolean) (IsFalling :type Boolean) (IsAttacking :type Boolean) (OsClimbing :type Boolean))
  (returns (OutputFB :type "PaperFlipbook Object Reference"))
  (locals (AnimationState :type "/Game/Data/AnimationState Enum"))
  (bind _climbinggirl (`self.ClimbingGirl`))
  (if OsClimbing
    (set `local.AnimationState` "NewEnumerator3")
    (elif IsAttacking
      (set `local.AnimationState` "NewEnumerator2")
      (elif IsFalling
        (set `local.AnimationState` "NewEnumerator4")
        (elif IsMoving
          (set `local.AnimationState` "NewEnumerator1")
          (else
            (set `local.AnimationState` "NewEnumerator0"))))))
  (return (select `/Game/Data/AnimationState` (`local.AnimationState`) :`NewEnumerator0` _climbinggirl :`NewEnumerator1` (`self.RunGirl`) :`NewEnumerator2` _climbinggirl :`NewEnumerator3` _climbinggirl :`NewEnumerator4` _climbinggirl)))

(fn `UserConstructionScript`)