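; FloorElement is a 2D floor piece built from Paper2D sprites, sized by the X distance between FloorLeft and FloorRight.
; The construction script lays a row of off-state sprites at RungOffset spacing, then scales and shifts Box along X using the span divided by X.
; SwitchState adds a second row of on-state sprites at the same positions, without removing the off-state ones.
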(event `self.ReceiveTick`
  (params (DeltaSeconds :type "Float (single-precision)")))

(fn `SwitchState`
  (bind _rungoffset (`self.RungOffset`))
  (bind _returnvalue_x (`KismetMathLibrary.BreakVector` (- (`self.FloorRight`) (`self.FloorLeft`))))
  (for _index (range (+ (`KismetMathLibrary.FTrunc` (/ _returnvalue_x _rungoffset)) 1))
    (bind _returnvalue (`AddComponent|NODE_AddPaperSpriteComponent-8` :`RelativeTransform` (`KismetMathLibrary.MakeTransform` (`KismetMathLibrary.MakeVector` (* _index _rungoffset)))))
    (`PaperSpriteComponent.SetSprite` _returnvalue (`self.OnSprite`))))

(fn `UserConstructionScript`
  (bind _box (`self.Box`))
  (bind _rungoffset (`self.RungOffset`))
  (bind _returnvalue_x (`KismetMathLibrary.BreakVector` (- (`self.FloorRight`) (`self.FloorLeft`))))
  (bind _returnvalue (/ _returnvalue_x (`self.X`)))
  (for _index (range (+ (`KismetMathLibrary.FTrunc` (/ _returnvalue_x _rungoffset)) 1))
    (bind _returnvalue_2 (`AddComponent|NODE_AddPaperSpriteComponent-6` :`RelativeTransform` (`KismetMathLibrary.MakeTransform` (`KismetMathLibrary.MakeVector` (* _index _rungoffset)))))
    (`PaperSpriteComponent.SetSprite` _returnvalue_2 (`self.OffSprite`)))
  (`SceneComponent.SetRelativeScale3D` _box (`KismetMathLibrary.MakeVector` _returnvalue 1.0 1.0))
  (`SceneComponent.K2_AddRelativeLocation` _box (`KismetMathLibrary.MakeVector` _returnvalue 1.0 1.0) false false))