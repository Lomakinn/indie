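; WallElement builds a vertical wall element from stacked Paper2D sprites, with an off and an on appearance.
; The construction script spawns off sprites every RungOffset along the Top-to-Bottom height, then scales and offsets Box from that height.
; SwitchState spawns a second stack with the on sprite at the same offsets, without removing existing sprites or providing a switch back.
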(event `self.ReceiveTick`
  (params (DeltaSeconds :type "Float (single-precision)")))

(fn `SwitchState`
  (bind _rungoffset (`self.RungOffset`))
  (bind (_returnvalue_x _returnvalue_y _returnvalue_z) (`KismetMathLibrary.BreakVector` (- (`self.Top`) (`self.Bottom`))))
  (for _index (range (+ (`KismetMathLibrary.FTrunc` (/ _returnvalue_z _rungoffset)) 1))
    (bind _returnvalue (`AddComponent|NODE_AddPaperSpriteComponent-8` :`RelativeTransform` (`KismetMathLibrary.MakeTransform` (`KismetMathLibrary.MakeVector` 0.0 0.0 (* _index _rungoffset)))))
    (`PaperSpriteComponent.SetSprite` _returnvalue (`self.OnSprite`))))

(fn `UserConstructionScript`
  (bind _box (`self.Box`))
  (bind _rungoffset (`self.RungOffset`))
  (bind (_returnvalue_x _returnvalue_y _returnvalue_z) (`KismetMathLibrary.BreakVector` (- (`self.Top`) (`self.Bottom`))))
  (bind _returnvalue (/ _returnvalue_z (`self.X`)))
  (for _index (range (+ (`KismetMathLibrary.FTrunc` (/ _returnvalue_z _rungoffset)) 1))
    (bind _returnvalue_2 (`AddComponent|NODE_AddPaperSpriteComponent-6` :`RelativeTransform` (`KismetMathLibrary.MakeTransform` (`KismetMathLibrary.MakeVector` 0.0 0.0 (* _index _rungoffset)))))
    (`PaperSpriteComponent.SetSprite` _returnvalue_2 (`self.OffSprite`)))
  (`SceneComponent.SetRelativeScale3D` _box (`KismetMathLibrary.MakeVector` 1.0 1.0 _returnvalue))
  (`SceneComponent.K2_AddRelativeLocation` _box (`KismetMathLibrary.MakeVector` 1.0 1.0 _returnvalue) false false))